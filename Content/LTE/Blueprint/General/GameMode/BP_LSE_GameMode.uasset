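; BP_LSE_GameMode is a game mode that tracks connected player controllers and spawns their characters.
; Login, controller-swap and logout events keep the AllPCs list updated.
; Spawn destroys a controller's current pawn, then spawns and possesses the CharClass stored in its LSE_Player_State at a randomly chosen PlayerStart, printing the new actor's name.
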(event `self.K2_PostLogin`
  (params (NewPlayer :type "PlayerController Object Reference"))
  (`KismetArrayLibrary.Array_Add` (`self.All PC's`) NewPlayer))

(event `self.K2_OnSwapPlayerControllers`
  (params (OldPC :type "PlayerController Object Reference") (NewPC :type "PlayerController Object Reference"))
  (`KismetArrayLibrary.Array_Add` (`self.All PC's`) NewPC))

(event `self.K2_OnLogout`
  (params (ExitingController :type "Controller Object Reference"))
  (bind _asbp_lse_player_controller (cast `/Game/LTE/Blueprint/General/Controller/BP_LSE_Player_Controller` ExitingController))
  (`KismetArrayLibrary.Array_RemoveItem` (`self.All PC's`) _asbp_lse_player_controller))

(fn `PlayerStart_Transform`
  (returns (ReturnValue :type "Transform Structure (by ref)"))
  (bind _outactors (`GameplayStatics.GetAllActorsOfClass` "/Script/Engine.PlayerStart"))
  (return (`self.GetTransform` (`|GetArrayItem` _outactors (`KismetMathLibrary.RandomIntegerInRange` 0 (- (`KismetArrayLibrary.Array_Length` _outactors) 1))))))

(fn `Spawn`
  (params (Controller :type "Controller Object Reference"))
  (bind _returnvalue (`Controller.K2_GetPawn` Controller))
  (`/Engine/EditorBlueprintResources/StandardMacros.IsValid` _returnvalue
    (:`Is Valid`
      (`self.K2_DestroyActor` _returnvalue))
    (:`Is Not Valid`
      _))
  (bind _returnvalue_2 (`|SpawnActorFromClass` (`/Game/LTE/Blueprint/General/PlayerState/LSE_Player_State.Char_Class` (cast `/Game/LTE/Blueprint/General/PlayerState/LSE_Player_State` (`Controller.PlayerState` Controller) :!pure true)) (`self.PlayerStart_Transform`) "AdjustIfPossibleButAlwaysSpawn" "OverrideRootScale" null null))
  (`Controller.Possess` Controller _returnvalue_2)
  (`KismetSystemLibrary.PrintString` (`KismetSystemLibrary.GetDisplayName` _returnvalue_2)))

(fn `UserConstructionScript`)