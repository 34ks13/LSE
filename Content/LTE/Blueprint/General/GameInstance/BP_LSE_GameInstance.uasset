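; Game instance that handles character selection among five playable characters and saves the chosen class.
; Cam_Change blends the player's view to the camera matching an index and stores that character's Blueprint class in CharPawn.
; Accept_Char writes CharPawn into the existing "Info" save slot, doing nothing if it fails to load.
; Init creates a save object in memory but never writes it to disk.
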(event `self.ReceiveInit`
  (bind _returnvalue (`GameplayStatics.CreateSaveGameObject` "/Game/LTE/Blueprint/General/SaveGame/BP_LSE_Save_CharInfo.BP_LSE_Save_CharInfo_C"))
  (set `self.Save_CharInfo` _returnvalue))

(event `Accept_Char`
  (bind _returnvalue (`GameplayStatics.LoadGameFromSlot` "Info"))
  (bind _asbp_lse_save_char_info (cast `/Game/LTE/Blueprint/General/SaveGame/BP_LSE_Save_CharInfo` _returnvalue))
  (set `/Game/LTE/Blueprint/General/SaveGame/BP_LSE_Save_CharInfo.Char_Class` (`self.Char_Pawn`) _asbp_lse_save_char_info)
  (`GameplayStatics.SaveGameToSlot` _asbp_lse_save_char_info "Info"))

(event `Cam_Change`
  (params (Index :type Integer))
  (switch `int` Index
    (:`1`
      (`PlayerController.SetViewTargetWithBlend` (`GameplayStatics.GetPlayerController` 0) (`self.DizzyCam`) 0.5 "VTBlend_Linear" 0.0 false)
      (set `self.Char_Pawn` "/Game/LTE/Blueprint/Character/BP_Dizzy.BP_Dizzy_C"))
    (:`2`
      (`PlayerController.SetViewTargetWithBlend` (`GameplayStatics.GetPlayerController` 0) (`self.RoyCam`) 0.5 "VTBlend_Linear" 0.0 false)
      (set `self.Char_Pawn` "/Game/LTE/Blueprint/Character/BP_Roy.BP_Roy_C"))
    (:`3`
      (`PlayerController.SetViewTargetWithBlend` (`GameplayStatics.GetPlayerController` 0) (`self.EmmaCam`) 0.5 "VTBlend_Linear" 0.0 false)
      (set `self.Char_Pawn` "/Game/LTE/Blueprint/Character/BP_Emma.BP_Emma_C"))
    (:`4`
      (`PlayerController.SetViewTargetWithBlend` (`GameplayStatics.GetPlayerController` 0) (`self.VolodyaCam`) 0.5 "VTBlend_Linear" 0.0 false)
      (set `self.Char_Pawn` "/Game/LTE/Blueprint/Character/BP_Volodya.BP_Volodya_C"))
    (:`5`
      (`PlayerController.SetViewTargetWithBlend` (`GameplayStatics.GetPlayerController` 0) (`self.AshbiCam`) 0.5 "VTBlend_Linear" 0.0 false)
      (set `self.Char_Pawn` "/Game/LTE/Blueprint/Character/BP_Ashby.BP_Ashby_C"))))