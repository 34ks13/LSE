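; Base weapon Blueprint that loads its settings from a DT_Weapon row in the construction script.
; Firing plays the pistol animation and a world camera shake, then runs Serv_Trace.
; Serv_Trace traces from player 0's camera to find the aim point, traces from the MuzzleFlash socket to it, and applies fixed damage to that hit actor.
; Loaded fire mode, rate, reload and spread values are not yet used, and TraceToCenter is empty.
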(event `/Game/LTE/Blueprint/General/Interface/BPI_Fire_Use.Fire_Use`
  (params (`Fire?` :type Boolean) (Char_Ref :type "/Game/LTE/Blueprint/Character/Base/LSE_Base_Character Object Reference"))
  (if `Fire?`
    (`self.Good_Shooting`)))

(event `Serv_Trace`
  (bind _returnvalue (`GameplayStatics.GetPlayerCameraManager` 0))
  (bind _returnvalue_2 (`SceneComponent.GetForwardVector` (`PlayerCameraManager.TransformComponent` _returnvalue)))
  (bind _returnvalue_3 (+ (`self.K2_GetActorLocation` _returnvalue) (* _returnvalue_2 250.0)))
  (bind _outhit (`KismetSystemLibrary.LineTraceSingle` :`Start` _returnvalue_3 :`End` (+ _returnvalue_3 (* _returnvalue_2 10000.0)) :`TraceChannel` "TraceTypeQuery1" :`DrawDebugType` "ForDuration" :`TraceColor` (struct :`G` 0.179179 :`B` 1.0 :`A` 1.0)))
  (bind _outhit_2 (`KismetSystemLibrary.LineTraceSingle` :`Start` (`SceneComponent.GetSocketLocation` (`self.Weapon`) "MuzzleFlash") :`End` (`.ImpactPoint` (`GameplayStatics.BreakHitResult` _outhit)) :`TraceChannel` "TraceTypeQuery1" :`DrawDebugType` "ForDuration"))
  (`GameplayStatics.ApplyDamage` (`.HitActor` (`GameplayStatics.BreakHitResult` _outhit_2)) 20.0))

(fn `Good_Shooting`
  (`SkeletalMeshComponent.PlayAnimation` (`self.Weapon`) "/Game/MilitaryWeapDark/Weapons/Anims/Fire_Pistol_W.Fire_Pistol_W" false)
  (`GameplayStatics.PlayWorldCameraShake` "/Game/LTE/Blueprint/Weapon/Cam_Shake/CS_Fire_Good.CS_Fire_Good_C" (`self.K2_GetActorLocation`) 0.0 500.0)
  (`self.Serv_Trace`))

(fn `Trace_To_Center`)

(fn `UserConstructionScript`
  (bind _returnvalue (`|GetDataTableRow` "/Game/LTE/Blueprint/Weapon/DT_Weapon.DT_Weapon" (`self.Weapon_Row_Name`))
    (:`then`
      (bind _output_get (set `self.Weapon_Data` _returnvalue))
      (bind (_firemode _muzzlename _firerate _reloaddelay _weaponspread) (break `/Game/LTE/Blueprint/Weapon/S_Weapon_Data` _output_get))
      (set `self.Fire Mode` _firemode)
      (set `self.Muzzle Name` _muzzlename)
      (set `self.Fire Rate` _firerate)
      (set `self.Reload Delay` _reloaddelay)
      (set `self.Weapon Spread` _weaponspread))))